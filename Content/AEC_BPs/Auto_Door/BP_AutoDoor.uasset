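; BP_AutoDoor is a sliding double door that opens when an actor overlaps it and closes when the overlap ends.
; The construction script caches each panel's relative Y as its closed position.
; An OpenDoors timeline, played on begin overlap and reversed on end overlap, lerps the two panels apart along local Y by a fixed offset.
; Overlaps are neither filtered nor counted, so any departing actor starts closing the doors.
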(event EventBeginPlay)

(event Collision|EventActorBeginOverlap
  (params (OtherActor :type Actor%20Object%20Reference))
  (bind _doorl_start (Variables|Default|GetDoorL_Start))
  (bind _autodoor_l (Variables|Default|GetAutoDoor_L))
  (bind _autodoor_r (Variables|Default|GetAutoDoor_R))
  (bind _doorr_start (Variables|Default|GetDoorR_Start))
  (bind _returnvalue (Transformation|GetRelativeTransform _autodoor_l))
  (bind _returnvalue_2 (Transformation|GetRelativeTransform _autodoor_r))
  (bind _open (Timeline|OpenDoors Play)
    (:Update
      (Transformation|SetRelativeLocation _autodoor_l (Math|Vector|MakeVector (.x (.location _returnvalue)) (Math|Float|Lerp _doorl_start (- _doorl_start 9e+01) _open) (.z (.location _returnvalue))) false false)
      (Transformation|SetRelativeLocation _autodoor_r (Math|Vector|MakeVector (.x (.location _returnvalue_2)) (Math|Float|Lerp _doorr_start (+ _doorr_start 9e+01) _open) (.z (.location _returnvalue_2))) false false))))

(event EventTick
  (params (DeltaSeconds :type Float%20%28single-precision%29)))

(event Collision|EventActorEndOverlap
  (params (OtherActor :type Actor%20Object%20Reference))
  (bind _doorl_start (Variables|Default|GetDoorL_Start))
  (bind _autodoor_l (Variables|Default|GetAutoDoor_L))
  (bind _autodoor_r (Variables|Default|GetAutoDoor_R))
  (bind _doorr_start (Variables|Default|GetDoorR_Start))
  (bind _returnvalue (Transformation|GetRelativeTransform _autodoor_l))
  (bind _returnvalue_2 (Transformation|GetRelativeTransform _autodoor_r))
  (bind _open (Timeline|OpenDoors Reverse)
    (:Update
      (Transformation|SetRelativeLocation _autodoor_l (Math|Vector|MakeVector (.x (.location _returnvalue)) (Math|Float|Lerp _doorl_start (- _doorl_start 9e+01) _open) (.z (.location _returnvalue))) false false)
      (Transformation|SetRelativeLocation _autodoor_r (Math|Vector|MakeVector (.x (.location _returnvalue_2)) (Math|Float|Lerp _doorr_start (+ _doorr_start 9e+01) _open) (.z (.location _returnvalue_2))) false false))))

(fn ConstructionScript
  (Variables|Default|SetDoorL_Start (.y (.location (Transformation|GetRelativeTransform (Variables|Default|GetAutoDoor_L)))))
  (Variables|Default|SetDoorR_Start (.y (.location (Transformation|GetRelativeTransform (Variables|Default|GetAutoDoor_R))))))